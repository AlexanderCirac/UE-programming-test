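; Game mode that tracks play time and player health in the game level and enforces a two-minute time limit.
; On BeginPlay it resets the stored time and health in Game_Instance_BP when the level is Niv_Juego_BP.
; Each Tick it reads elapsed game time, copies minutes, seconds and ThirdPersonCharacter health into the game instance, and opens Niv_Perder_BP, the lose level, once time runs out.
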(event `self.ReceiveBeginPlay`
  (`self.ReiniciarDartos`))

(event `self.ReceiveTick`
  (params (DeltaSeconds :type "Float (single-precision)"))
  (`self.M_Contar_Tiempo`)
  (`self.GuardarDatos`)
  (`self.morir_por_Tiempo`))

(event `M_Contar_Tiempo`
  (bind _returnvalue (`GameplayStatics.GetCurrentLevelName` true))
  (if (`KismetStringLibrary.EqualEqual_StrStr` _returnvalue "Niv_Juego_BP")
    (bind _output_get (set `self.var_tiempoJugado` (`KismetSystemLibrary.GetGameTimeInSeconds`)))))

(event `GuardarDatos`
  (bind _returnvalue (`GameplayStatics.GetCurrentLevelName` true))
  (if (`KismetStringLibrary.EqualEqual_StrStr` _returnvalue "Niv_Juego_BP")
    (bind _asgame_instance_bp (cast `/Game/Juego/Programing_BP/Game_Instance_BP` (`GameplayStatics.GetGameInstance`)))
    (bind (_days _hours _minutes _seconds) (`KismetMathLibrary.BreakTimespan` (`KismetMathLibrary.TimespanFromString` (`KismetStringLibrary.TimeSecondsToString` (stale `M_Contar_Tiempo` _output_get)))))
    (set `/Game/Juego/Programing_BP/Game_Instance_BP.var_int_tiempo_Min` _minutes _asgame_instance_bp)
    (set `/Game/Juego/Programing_BP/Game_Instance_BP.var_int_tiempo_Seg` _seconds _asgame_instance_bp)
    (bind _asthird_person_character (cast `/Game/ThirdPersonCPP/Blueprints/ThirdPersonCharacter` (`GameplayStatics.GetPlayerCharacter` 0)))
    (set `/Game/Juego/Programing_BP/Game_Instance_BP.var_Vida` (`Prueba_TrooperBLackCharacter.var_vida` _asthird_person_character) _asgame_instance_bp)))

(event `ReiniciarDartos`
  (bind _returnvalue (`GameplayStatics.GetCurrentLevelName` true))
  (if (`KismetStringLibrary.EqualEqual_StrStr` _returnvalue "Niv_Juego_BP")
    (bind _asgame_instance_bp (cast `/Game/Juego/Programing_BP/Game_Instance_BP` (`GameplayStatics.GetGameInstance`)))
    (set `/Game/Juego/Programing_BP/Game_Instance_BP.var_int_tiempo_Min` 0 _asgame_instance_bp)
    (set `/Game/Juego/Programing_BP/Game_Instance_BP.var_int_tiempo_Seg` 0 _asgame_instance_bp)
    (set `/Game/Juego/Programing_BP/Game_Instance_BP.var_Vida` 100.0 _asgame_instance_bp)))

(event `morir_por_Tiempo`
  (if (>= (`self.var_tiempoJugado`) 120.0)
    (`GameplayStatics.OpenLevel` "Niv_Perder_BP")))

(fn `UserConstructionScript`)