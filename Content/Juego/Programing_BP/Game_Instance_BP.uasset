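; Game instance Blueprint that acts as a simple text localization lookup for the game.
; F_Lector_Texto takes a text index and picks the string from the Castilian Spanish or English array according to the language ID variable.
; IDs of 1 or below select Spanish and higher ones English; the string is stored as the current text and returned as Text.
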(fn `F_Lector_Texto`
  (params (var_Int_Texto :type Integer))
  (returns (var_Str_texto :type Text))
  (bind _var_int_id_idioma (`self.var_Int_ID_Idioma`))
  (`|ExecutionSequence`
    (:`then_0`
      (if (<= _var_int_id_idioma 1)
        (set `self.var_Str_TextoActual` (`|GetArrayItem` (`self.var_Str_Castellano`) var_Int_Texto))
        (return (`KismetTextLibrary.Conv_StringToText` (`self.var_Str_TextoActual`)))))
    (:`then_1`
      (if (>= _var_int_id_idioma 2)
        (set `self.var_Str_TextoActual` (`|GetArrayItem` (`self.var_Str_Ingles`) var_Int_Texto))
        (return (`KismetTextLibrary.Conv_StringToText` (`self.var_Str_TextoActual`)))))))