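; Destructible barrier actor that loses health when hit by bullets and destroys itself once health runs out.
; A trigger overlap with a "Bala"-tagged bullet subtracts that bullet's damage and spawns a floating damage number projected from the cube's position to screen space.
; A sphere overlap shows or hides the health widget as the player character enters or leaves.
; Tick refreshes the health bar and checks for destruction.
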(event `self.ReceiveTick`
  (params (DeltaSeconds :type "Float (single-precision)"))
  (`self.Decir_Info`)
  (if (<= (`self.var_vida`) 0.0)
    (`self.K2_DestroyActor`)))

(event `self.Sphere.OnComponentBeginOverlap`
  (params (OverlappedComponent :type "PrimitiveComponent Object Reference") (OtherActor :type "Actor Object Reference") (OtherComp :type "PrimitiveComponent Object Reference") (OtherBodyIndex :type Integer) (bFromSweep :type Boolean) (SweepResult :type "HitResult Structure (by ref)"))
  (cast `/Game/ThirdPersonCPP/Blueprints/ThirdPersonCharacter` OtherActor)
  (`SceneComponent.SetVisibility` (`self.Widget`) true false))

(event `self.Sphere.OnComponentEndOverlap`
  (params (OverlappedComponent :type "PrimitiveComponent Object Reference") (OtherActor :type "Actor Object Reference") (OtherComp :type "PrimitiveComponent Object Reference") (OtherBodyIndex :type Integer))
  (cast `/Game/ThirdPersonCPP/Blueprints/ThirdPersonCharacter` OtherActor)
  (`SceneComponent.SetVisibility` (`self.Widget`) false false))

(event `self.Trigger.OnComponentBeginOverlap`
  (params (OverlappedComponent :type "PrimitiveComponent Object Reference") (OtherActor :type "Actor Object Reference") (OtherComp :type "PrimitiveComponent Object Reference") (OtherBodyIndex :type Integer) (bFromSweep :type Boolean) (SweepResult :type "HitResult Structure (by ref)"))
  (if (`self.ActorHasTag` OtherActor "Bala")
    (bind _asobjeto_bala_bp (cast `/Game/Juego/Programing_BP/Objetos_BP/Objeto_bala_BP` OtherActor))
    (bind `_var_daño` (`/Game/Juego/Programing_BP/Objetos_BP/Objeto_bala_BP.var_Daño` _asobjeto_bala_bp))
    (set `self.var_vida` (- (`self.var_vida`) `_var_daño`))
    (`self.Daño_flotante` (`SceneComponent.K2_GetComponentLocation` (`self.Cube`)) `_var_daño`)))

(event `Decir_Info`
  (bind _aswidget_nivel_juego_objetos_bp (cast `/Game/Juego/Programing_BP/Widget_BP/Widget_NivelJuego_Objetos_BP` (`WidgetComponent.GetUserWidgetObject` (`self.Widget`))))
  (`ProgressBar.SetPercent` (`/Game/Juego/Programing_BP/Widget_BP/Widget_NivelJuego_Objetos_BP.ProgressBar_Vida_Objeto` _aswidget_nivel_juego_objetos_bp) (/ (`self.var_vida`) 100.0)))

(fn `Daño_flotante`
  (params (var_SpawnPosicion :type "Vector Structure") (`var_daño` :type "Float (double-precision)"))
  (bind _returnvalue (`|CreateWidget` "/Game/Juego/Programing_BP/Widget_BP/Widget_NumeroDaño_BP.Widget_NumeroDaño_BP_C" null `var_daño` (`GameplayStatics.ProjectWorldToScreen` (`GameplayStatics.GetPlayerController` 0) var_SpawnPosicion true)))
  (`UserWidget.AddToViewport` _returnvalue 0))

(fn `UserConstructionScript`)