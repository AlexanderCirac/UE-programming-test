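; Harmful wall variant of a destructible barrier that hurts the player on contact.
; Entering the TriggerDaño volume subtracts a fixed amount directly from VarVida in the ThirdPersonCharacter's health component.
; A DoOnce limits this to one hit until the character leaves the trigger; it sits before the cast, so another overlapping actor can consume it.
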(event `self.TriggerDaño.OnComponentBeginOverlap`
  (params (OverlappedComponent :type "PrimitiveComponent Object Reference") (OtherActor :type "Actor Object Reference") (OtherComp :type "PrimitiveComponent Object Reference") (OtherBodyIndex :type Integer) (bFromSweep :type Boolean) (SweepResult :type "HitResult Structure (by ref)"))
  (`/Engine/EditorBlueprintResources/StandardMacros.DoOnce` false :!label _label
    (:`Completed`
      (bind _asthird_person_character (cast `/Game/ThirdPersonCPP/Blueprints/ThirdPersonCharacter` OtherActor))
      (bind _component_vida_jugador_bp (`/Game/ThirdPersonCPP/Blueprints/ThirdPersonCharacter.Component_Vida_Jugador_BP` _asthird_person_character))
      (set `/Game/Juego/Programing_BP/Objetos_BP/Component_Vida_Jugador_BP.var_vida` (- (`/Game/Juego/Programing_BP/Objetos_BP/Component_Vida_Jugador_BP.var_vida` _component_vida_jugador_bp) 30.0) _component_vida_jugador_bp))))

(event `self.TriggerDaño.OnComponentEndOverlap`
  (params (OverlappedComponent :type "PrimitiveComponent Object Reference") (OtherActor :type "Actor Object Reference") (OtherComp :type "PrimitiveComponent Object Reference") (OtherBodyIndex :type Integer))
  (cast `/Game/ThirdPersonCPP/Blueprints/ThirdPersonCharacter` OtherActor)
  (goto _label :!via `Reset`))

(fn `UserConstructionScript`
  (`parent.UserConstructionScript`))