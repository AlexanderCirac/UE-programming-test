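; Victory circle actor that wins the game once the player has collected all required items.
; Every Tick it shows or hides its Sphere depending on whether the collection counter in Game_Mode_BP equals seven.
; When a ThirdPersonCharacter overlaps the Sphere with that count reached, the Victoria event opens the Niv_Ganar_BP level.
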(event `self.ReceiveTick`
  (params (DeltaSeconds :type "Float (single-precision)"))
  (`self.Activar_Visiblididad`))

(event `self.Sphere.OnComponentBeginOverlap`
  (params (OverlappedComponent :type "PrimitiveComponent Object Reference") (OtherActor :type "Actor Object Reference") (OtherComp :type "PrimitiveComponent Object Reference") (OtherBodyIndex :type Integer) (bFromSweep :type Boolean) (SweepResult :type "HitResult Structure (by ref)"))
  (bind _asgame_mode_bp (cast `/Game/Juego/Programing_BP/Game_Mode_BP` (`GameplayStatics.GetGameMode`)))
  (if (== 7 (`/Game/Juego/Programing_BP/Game_Mode_BP.var_intRecoleccion` _asgame_mode_bp))
    (cast `/Game/ThirdPersonCPP/Blueprints/ThirdPersonCharacter` OtherActor)
    (`self.Victoria`)))

(event `Victoria`
  (`GameplayStatics.OpenLevel` "Niv_Ganar_BP"))

(event `Activar_Visiblididad`
  (bind _asgame_mode_bp (cast `/Game/Juego/Programing_BP/Game_Mode_BP` (`GameplayStatics.GetGameMode`)))
  (if (== (`/Game/Juego/Programing_BP/Game_Mode_BP.var_intRecoleccion` _asgame_mode_bp) 7)
    (`SceneComponent.SetVisibility` (`self.Sphere`) true false)
    (else
      (`SceneComponent.SetVisibility` (`self.Sphere`) false false))))

(fn `UserConstructionScript`)