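; Collectible objective pickup that bobs up and down and adds to the game's collection count.
; BeginPlay stores the body's world position, and Tick moves it along local Z, reversing direction at fixed limits above and below that start.
; When a ThirdPersonCharacter overlaps the trigger, it increments the collection counter on Game_Mode_BP, then destroys itself.
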(event `Guardar Posicion`
  ;[1 1 1] Guardamos posicion incialmente
  (set `self.var_vec3` (`SceneComponent.K2_GetComponentLocation` (`self.Cuerpo`))))

(event `self.ReceiveBeginPlay`
  (`self.Guardar Posicion`))

(event `mirar_posicion_acutal`
  (bind (_var_vec3_x _var_vec3_y _var_vec3_z) (`KismetMathLibrary.BreakVector` (`self.var_vec3`)))
  (bind (_var_vec3_x_2 _var_vec3_y_2 _var_vec3_z_2) (`KismetMathLibrary.BreakVector` (`self.var_vec3`)))
  (bind (_returnvalue_x _returnvalue_y _returnvalue_z) (`KismetMathLibrary.BreakVector` (`SceneComponent.K2_GetComponentLocation` (`self.Cuerpo`))))
  (bind (_returnvalue_x_2 _returnvalue_y_2 _returnvalue_z_2) (`KismetMathLibrary.BreakVector` (`SceneComponent.K2_GetComponentLocation` (`self.Cuerpo`))))
  ;[1 1 1] Control de posicion actual
  (`|ExecutionSequence`
    (:`then_0`
      (if (>= _returnvalue_z_2 (+ _var_vec3_z 40.0))
        (set `self.var_pos` false)))
    (:`then_1`
      (if (<= _returnvalue_z (- _var_vec3_z_2 40.0))
        (set `self.var_pos` true)))))

(event `self.ReceiveTick`
  (params (DeltaSeconds :type "Float (single-precision)"))
  (`self.mirar_posicion_acutal`)
  (`self.Animacion_posicion`))

(event `self.trigger.OnComponentBeginOverlap`
  (params (OverlappedComponent :type "PrimitiveComponent Object Reference") (OtherActor :type "Actor Object Reference") (OtherComp :type "PrimitiveComponent Object Reference") (OtherBodyIndex :type Integer) (bFromSweep :type Boolean) (SweepResult :type "HitResult Structure (by ref)"))
  (cast `/Game/ThirdPersonCPP/Blueprints/ThirdPersonCharacter` OtherActor)
  (`self.Recolecion`)
  (`self.K2_DestroyActor`))

(event `Animacion_posicion`
  (bind _cuerpo (`self.Cuerpo`))
  ;[1 1 1] Animacion
  (if (`self.var_pos`)
    (`SceneComponent.K2_AddLocalOffset` _cuerpo (0.0 0.0 2.0) false false)
    (else
      (`SceneComponent.K2_AddLocalOffset` _cuerpo (0.0 0.0 -2.0) false false))))

(event `Recolecion`
  ;[1 1 1] Sumar los objetos recolectables
  (bind _asgame_mode_bp (cast `/Game/Juego/Programing_BP/Game_Mode_BP` (`GameplayStatics.GetGameMode`)))
  (set `/Game/Juego/Programing_BP/Game_Mode_BP.var_intRecoleccion` (+ (`/Game/Juego/Programing_BP/Game_Mode_BP.var_intRecoleccion` _asgame_mode_bp) 1) _asgame_mode_bp))

(fn `UserConstructionScript`)